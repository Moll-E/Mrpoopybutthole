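; Player controller that drives the first ship in a two-ship twin-stick setup and spawns the second ship.
; Left-ship axis inputs move the controlled pawn along forward and right vectors derived from its control rotation.
; On BeginPlay it spawns a second Joycon controller and a TwinStickPawn21 at a fixed location, stores both, and has that controller possess the new pawn.
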(event EventBeginPlay
  (bind _returnvalue (Math|Transform|MakeTransform "-840.000000,700.000000,220.000000"))
  ;[1 1 1] Ship 2 spawn
  (bind _returnvalue_2 (Game|SpawnActorfromClass "/Game/Blueprints/JoyconTwoPlayerController.JoyconTwoPlayerController_C" _returnvalue "Undefined" 0 0))
  (Variables|Default|SetRight%20Ship%20Control _returnvalue_2)
  (bind _returnvalue_3 (Game|SpawnActorfromClass "/Game/Blueprints/TwinStickBP/Blueprints/TwinStickPawn21.TwinStickPawn21_C" _returnvalue "Undefined" 0 0))
  (Variables|Default|SetRight%20Ship _returnvalue_3)
  (Pawn|Possess (Variables|Default|GetRight%20Ship%20Control) (Variables|Default|GetRight%20Ship)))

(event Input|AxisEvents|InputAxisMovementLShipFoward
  (params (AxisValue :type Float%20%28single-precision%29))
  (bind _returnvalue (Pawn|GetControlledPawn))
  ;[1 1 1] Ship 1 movement
  (Pawn|Input|AddMovementInput _returnvalue (Math|Vector|GetForwardVector (Pawn|GetControlRotation _returnvalue :!class /Script/Engine.Pawn)) AxisValue false))

(event Input|AxisEvents|InputAxisMovementLShipRight
  (params (AxisValue :type Float%20%28single-precision%29))
  (bind _returnvalue (Pawn|GetControlledPawn))
  ;[1 1 1] Ship 1 movement
  (Pawn|Input|AddMovementInput _returnvalue (Math|Vector|GetRightVector (Pawn|GetControlRotation _returnvalue :!class /Script/Engine.Pawn)) AxisValue false))

(fn ConstructionScript)